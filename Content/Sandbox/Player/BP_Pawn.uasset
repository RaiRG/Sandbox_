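; BP_Pawn is a sandbox player pawn that handles movement and a dance-switch input through Enhanced Input.
; On BeginPlay it registers IMC_Default with the player controller, and IA_Move feeds movement input along the actor's right and forward vectors.
; IA_DanceSwitch holds the NeedSwitchAnimation flag true while pressed; nothing in this Blueprint reads it.
; Controller look and world-offset nodes are present but disconnected, so they never run.
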(event `self.ReceiveBeginPlay`
  (bind _asplayer_controller (cast `PlayerController` (`self.GetController`)))
  (message `EnhancedInputSubsystemInterface.AddMappingContext` (pcsubsystem `EnhancedInputLocalPlayerSubsystem` _asplayer_controller) "/Game/Sandbox/Player/IMC_Default.IMC_Default" 0 (struct)))

(event `EnhancedInput|/Game/Sandbox/Player/IA_Move`
  (params (ActionValue :type "Vector2D Structure") (ElapsedSeconds :type "Float (double-precision)") (TriggeredSeconds :type "Float (double-precision)") (InputAction :type "InputAction Object Reference" :default "/Game/Sandbox/Player/IA_Move.IA_Move"))
  (:`Triggered`
    (if (not (`KismetMathLibrary.NearlyEqual_FloatFloat` ActionValue_X))
      (`self.AddMovementInput` (`self.GetActorRightVector`) ActionValue_X))
    (if (not (`KismetMathLibrary.NearlyEqual_FloatFloat` ActionValue_Y))
      (`self.AddMovementInput` (`self.GetActorForwardVector`) ActionValue_Y))))

(event `EnhancedInput|/Game/Sandbox/Player/IA_DanceSwitch`
  (params (ActionValue :type Boolean) (ElapsedSeconds :type "Float (double-precision)") (TriggeredSeconds :type "Float (double-precision)") (InputAction :type "InputAction Object Reference" :default "/Game/Sandbox/Player/IA_DanceSwitch.IA_DanceSwitch"))
  (:`Started`
    (set `self.NeedSwitchAnimation` true))
  (:`Completed`
    (set `self.NeedSwitchAnimation` false)))

(event `EnhancedInput|/Game/Sandbox/Player/IA_Turn`
  (params (ActionValue :type "Vector2D Structure") (ElapsedSeconds :type "Float (double-precision)") (TriggeredSeconds :type "Float (double-precision)") (InputAction :type "InputAction Object Reference" :default "/Game/Sandbox/Player/IA_Turn.IA_Turn")))

(fn `UserConstructionScript`)